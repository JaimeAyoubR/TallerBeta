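; BP_Lava is a lava actor that rises vertically over time.
; On Tick, while MaxZPos is true, it moves up along Z by VelocidadSubida scaled by world delta seconds, without sweep.
; When the flag is false, it holds position for that tick and sets the flag true, so no height limit is enforced here.
; BeginPlay, overlap and construction logic are empty.
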(event `self.ReceiveTick`
  (params (DeltaSeconds :type "Float (single-precision)"))
  (if (`self.MaxZPos`)
    (`self.K2_SetActorLocation` (`KismetMathLibrary.MakeVector` (.x (`self.K2_GetActorLocation`)) (.y (`self.K2_GetActorLocation`)) (+ (.z (`self.K2_GetActorLocation`)) (* (`self.VelocidadSubida`) (`GameplayStatics.GetWorldDeltaSeconds`)))))
    (else
      (`self.K2_SetActorLocation` (`self.K2_GetActorLocation`))
      (set `self.MaxZPos` true))))

(fn `UserConstructionScript`)