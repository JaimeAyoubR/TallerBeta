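; BP_LavaHazard is a lava hazard actor that rises vertically and tracks players who touch it.
; While IsRising is set, Tick raises it at RiseSpeed until TargetHeight, printing its location each frame.
; Collider overlap with Player_BP stores the player and starts a looping timer for ApplyDamageTimer, cleared when that player leaves.
; ApplyDamageTimer is called by name but is not defined in these graphs.
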(event `self.ReceiveTick`
  (params (DeltaSeconds :type "Float (single-precision)"))
  (if (`self.IsRising `)
    (`self.K2_SetActorLocation` (+ (`self.K2_GetActorLocation`) (`KismetMathLibrary.MakeVector` 0.0 0.0 (* (`self.RiseSpeed `) DeltaSeconds))))
    (`KismetSystemLibrary.PrintText` (`KismetTextLibrary.Conv_VectorToText` (`self.K2_GetActorLocation`)))
    (if (>= (.z (`self.K2_GetActorLocation`)) (`self.TargetHeight `))
      (set `self.IsRising ` false))
    (else
      (`self.K2_SetActorLocation` (`self.K2_GetActorLocation`)))))

(event `self.Collider.OnComponentBeginOverlap`
  (params (OverlappedComponent :type "PrimitiveComponent Object Reference") (OtherActor :type "Actor Object Reference") (OtherComp :type "PrimitiveComponent Object Reference") (OtherBodyIndex :type Integer) (bFromSweep :type Boolean) (SweepResult :type "HitResult Structure (by ref)"))
  (bind _asplayer_bp (cast `/Game/Taller/Blueprints/Player_BP` OtherActor))
  (set `self.OverlappingPlayer ` _asplayer_bp)
  (`KismetSystemLibrary.K2_SetTimer` null "ApplyDamageTimer" (`self.DamageInterval `) true))

(event `self.Collider.OnComponentEndOverlap`
  (params (OverlappedComponent :type "PrimitiveComponent Object Reference") (OtherActor :type "Actor Object Reference") (OtherComp :type "PrimitiveComponent Object Reference") (OtherBodyIndex :type Integer))
  (if (== OtherActor (`self.OverlappingPlayer `))
    (set `self.OverlappingPlayer ` null)
    (`KismetSystemLibrary.K2_ClearTimer` null "ApplyDamageTimer")))

(fn `UserConstructionScript`)