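; Bat hazard that flies back and forth along a straight path and damages the player on contact.
; On BeginPlay a looping linear yoyo vector tween runs between the start location and a Destination offset, with configurable duration and delay.
; Each tween update turns the bat toward the next position before moving it there without sweep.
; Overlapping the Trigger component calls TakeDamageEvent on Player_BP.
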(event `self.ReceiveBeginPlay`
  (bind _delaytween (`self.DelayTween`))
  (bind _output_get (set `self.StartLocation` (`self.K2_GetActorLocation` self)))
  (bind (_asynctaskproxy _value) (`FCTweenBPActionVector.TweenVector` _output_get (+ (`self.StartLocation`) (`self.Destination`)) (`self.DurationTween`) "Linear" 0.0 0.0 _delaytween -1 _delaytween true _delaytween)
    (:`ApplyEasing`
      (`self.K2_SetActorRotation` (`KismetMathLibrary.FindLookAtRotation` (`self.K2_GetActorLocation`) _value))
      (`self.K2_SetActorLocation` self _value false false))))

(event `self.Trigger.OnComponentBeginOverlap`
  (params (OverlappedComponent :type "PrimitiveComponent Object Reference") (OtherActor :type "Actor Object Reference") (OtherComp :type "PrimitiveComponent Object Reference") (OtherBodyIndex :type Integer) (bFromSweep :type Boolean) (SweepResult :type "HitResult Structure (by ref)"))
  (bind _asplayer_bp (cast `/Game/Taller/Blueprints/Player_BP` OtherActor))
  (`/Game/Taller/Blueprints/Player_BP.TakeDamageEvent` _asplayer_bp))

(fn `UserConstructionScript`)